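; Boss enemy character that chases the player and plays an attack or skill montage on reaching them.
; PawnSensing sets a seen flag and, after a three-second delay, calls FollowPlayer, which uses AIMoveTo toward the player.
; On arrival, CurrentTime selects Attack while positive, otherwise Skill, then resets to MakeTime; nothing here counts it down.
; StartAttack holds an alternate timer comparison but is only called from unconnected nodes.
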(event `self.PawnSensing.OnSeePawn`
  (params (Pawn :type "Pawn Object Reference"))
  ;[1 1 1] 보스 감지 후 플레이어 따라가기
  (set `self.isSeeingPlayer` true)
  (`KismetSystemLibrary.Delay` 3.0)
  (`self.FollowPlayer`))

(event `FollowPlayer`
  ;[1 1 1] 보스 공격패턴(걸어갈 때 범위에 있으면 공격)
  (set `self.canAttack` true)
  (if (`self.isSeeingPlayer`)
    (`|AIMoveTo` self (0.0 0.0 0.0) (`GameplayStatics.GetPlayerCharacter` 0)
      (:`OnSuccess`
        (if (`self.canAttack`)
          (if (> (`self.CurrentTime`) 0.0)
            (`self.PlayAnimMontage` "/Game/animation/Attack_Montage.Attack_Montage")
            (`KismetSystemLibrary.PrintString` "Attack")
            (else
              (`self.PlayAnimMontage` "/Game/animation/skill_Montage.skill_Montage")
              (set `self.CurrentTime` (`self.MakeTime`))
              (`KismetSystemLibrary.PrintString` "Skill!"))))))))

(event `self.ReceiveTick`
  (params (DeltaSeconds :type "Float (single-precision)")))

(fn `StartAttack`
  (params (NewParam :type Boolean) (NewParam1 :type Boolean))
  (if (> (`self.CurrentTime`) (`self.MakeTime`))
    (`self.PlayAnimMontage` "/Game/animation/skill_Montage.skill_Montage")
    (`KismetSystemLibrary.PrintString` "Skill!")
    (else
      (`self.PlayAnimMontage` "/Game/animation/Attack_Montage.Attack_Montage")
      (`KismetSystemLibrary.PrintString` "Attack"))))

(fn `UserConstructionScript`)