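; BP_TestEnemy is a test enemy that chases the player when near and walks back to its spawn point beyond leash range.
; Tick dispatches on a State enum; Chase randomly picks melee or skill attacks by distance, though the wider skill check overwrites melee picks.
; Attacks share one accumulating timer with separate thresholds, playing an animation and debug print before resuming Chase.
; The Return state is empty and Hit is never called here.
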(event `self.ReceiveBeginPlay`
  ;[1 1 1] 일정 거리가 넘어가면 원래 자리로 되돌아 가기위한 위치 선정
  (set `self.return` (`self.K2_GetActorLocation`))
  (set `self.ChaseTarget` (`GameplayStatics.GetPlayerCharacter` 0)))

(event `EventStay`
  (bind _returnvalue (`GameplayStatics.GetPlayerCharacter` 0))
  ;[1 1 1] 내 반경 3M안에 플레이어가 있다면 추적 상태로 전이하고싶다.
  (set `self.ChaseTarget` _returnvalue)
  (if (< (`KismetMathLibrary.Vector_Distance` (`self.K2_GetActorLocation` _returnvalue) (`self.K2_GetActorLocation`)) 700.0)
    (set `self.State` "NewEnumerator0")))

(event `EventChase`
  ;[1 1 1] 목적지를 향해 이동하고싶다.
  (`AIBlueprintHelperLibrary.SimpleMoveToLocation` (`self.GetController`) (`self.K2_GetActorLocation` (`self.ChaseTarget`)))
  (if (> (`KismetMathLibrary.VSize` (- (`self.K2_GetActorLocation` (`GameplayStatics.GetPlayerCharacter` 0)) (`self.K2_GetActorLocation` self))) 1000.0)
    (`AIBlueprintHelperLibrary.SimpleMoveToLocation` (`self.GetController`) (`self.return`))
    (else
      (`|ExecutionSequence`
        (:`then_0`
          (if (> 200.0 (`KismetMathLibrary.VSize` (- (`self.K2_GetActorLocation` (`GameplayStatics.GetPlayerCharacter` 0)) (`self.K2_GetActorLocation` self))))
            (set `self.State` "NewEnumerator3")
            ;[1 1 1] 3중에 하나를 랜덤으로 공격하고 싶다.
            (switch `int` (`KismetMathLibrary.RandomIntegerInRange` 0 1)
              (:`0`
                (set `self.State` "NewEnumerator1"))
              (:`1`
                (set `self.State` "NewEnumerator5")))))
        (:`then_1`
          (if (> 500.0 (`KismetMathLibrary.VSize` (- (`self.K2_GetActorLocation` (`GameplayStatics.GetPlayerCharacter` 0)) (`self.K2_GetActorLocation` self))))
            (set `self.State` "NewEnumerator3")
            (switch `int` (`KismetMathLibrary.RandomIntegerInRange` 0 1)
              (:`0`
                (set `self.State` "NewEnumerator6"))
              (:`1`
                (set `self.State` "NewEnumerator8")))))))))

(event `EventReturn`)

(event `EventAttack`
  ;[1 1 1] 가까이 왔을 때 일반 공격하고 싶다.
  (bind _output_get (set `self.CurrentTime` (+ (`self.CurrentTime`) (`GameplayStatics.GetWorldDeltaSeconds`))))
  (if (> _output_get (`self.MakeTime1`))
    (`SkeletalMeshComponent.PlayAnimation` (`self.Mesh`) "/Game/animation/Attack1_Jab.Attack1_Jab" false)
    (set `self.CurrentTime` 0.0)
    (`KismetSystemLibrary.PrintString` "Attack")
    (set `self.State` "NewEnumerator0")
    (else
      (set `self.State` "NewEnumerator0"))))

(event `Power Attack`
  ;[1 1 1] 가까이 왔을 때 쌔게 때리고 싶다
  (bind _output_get (set `self.CurrentTime` (+ (`self.CurrentTime`) (`GameplayStatics.GetWorldDeltaSeconds`))))
  (if (> _output_get (`self.MakeTime2`))
    (`SkeletalMeshComponent.PlayAnimation` (`self.Mesh`) "/Game/animation/Attack2_Straight.Attack2_Straight" false)
    (set `self.CurrentTime` 0.0)
    (`KismetSystemLibrary.PrintString` "Power Attack")
    ;[1 1 1] 강 공격 중 공격을 받으면 잠깐 멈추고 싶다.
    (set `self.State` "NewEnumerator0")
    (else
      (set `self.State` "NewEnumerator0"))))

(event `self.ReceiveTick`
  (params (DeltaSeconds :type "Float (single-precision)"))
  (switch `/Game/Buleprints/EEnemyState` (`self.State`)
    (:`NewEnumerator3`
      (`self.EventStay`))
    (:`NewEnumerator0`
      (`self.EventChase`))
    (:`NewEnumerator4`
      (`self.EventReturn`))
    (:`NewEnumerator1`
      (`self.EventAttack`))
    (:`NewEnumerator5`
      (`self.Power Attack`))
    (:`NewEnumerator6`
      (`self.Skill`))
    (:`NewEnumerator8`
      (`self.jump skill`))))

(event `Skill`
  ;[1 1 1] 가까이 왔을 때 스킬을 쓰고 싶다.
  (bind _output_get (set `self.CurrentTime` (+ (`self.CurrentTime`) (`GameplayStatics.GetWorldDeltaSeconds`))))
  (if (> _output_get (`self.MakeTime3`))
    (`SkeletalMeshComponent.PlayAnimation` (`self.Mesh`) "/Game/animation/Attack3_Hook.Attack3_Hook" false)
    (set `self.CurrentTime` 0.0)
    (`KismetSystemLibrary.PrintString` "skill")
    (set `self.State` "NewEnumerator0")
    (else
      (set `self.State` "NewEnumerator0"))))

(event `jump skill`
  ;[1 1 1] 스킬(점프해서 적을 찍는 모션-> 일정거리 떨어져 있을 때)
  (bind _output_get (set `self.CurrentTime` (+ (`self.CurrentTime`) (`GameplayStatics.GetWorldDeltaSeconds`))))
  (if (> _output_get (`self.makeTime4`))
    (`SkeletalMeshComponent.PlayAnimation` (`self.Mesh`) "/Game/Characters/Mannequins/Animations/Manny/MM_Jump.MM_Jump" false)
    (set `self.CurrentTime` 0.0)
    (`KismetSystemLibrary.PrintString` "jump skill")
    (else
      (set `self.State` "NewEnumerator0"))))

(event `Hit`
  ;[1 1 1] 맞을 때의 반응을 하고 싶다.
  (if (`self.HitbyPlayer`)
    (`KismetSystemLibrary.Delay` 4.0)
    (set `self.State` "NewEnumerator0")
    (else
      (set `self.State` "NewEnumerator1"))))

(fn `NewFunction`)

(fn `UserConstructionScript`)