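; BP_SecondCharacter is a character Blueprint with an unfinished target lock-on system.
; The LockOnRadius overlaps maintain a list of candidate actors.
; Engagelock re-invokes itself every 0.1 seconds while engaged, setting control rotation along the target-to-character direction, and disengages when the target is invalid.
; The toggle logic that picks a target or swaps is unwired, and swaplock is empty.
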(event `self.ReceiveActorBeginOverlap`
  (params (OtherActor :type "Actor Object Reference")))

(event `disengagelock`
  (set `self.BlockOnEngaged` false)
  (set `self.LockOnIndex` 0))

(event `Engagelock`
  (bind _currenttarget (`self.CurrentTarget`)
    (:`then`
      (`Controller.SetControlRotation` (`GameplayStatics.GetPlayerController` 0) (`KismetMathLibrary.FindLookAtRotation` (`self.K2_GetActorLocation` _currenttarget) (`self.K2_GetActorLocation`)))
      (`KismetSystemLibrary.Delay` 0.1)
      (if (`self.BlockOnEngaged`)
        (`self.Engagelock`)))
    (:`else`
      (`self.disengagelock`))))

(event `swaplock`)

(event `self.LockOnRadius.OnComponentBeginOverlap`
  (params (OverlappedComponent :type "PrimitiveComponent Object Reference") (OtherActor :type "Actor Object Reference") (OtherComp :type "PrimitiveComponent Object Reference") (OtherBodyIndex :type Integer) (bFromSweep :type Boolean) (SweepResult :type "HitResult Structure (by ref)"))
  (`KismetArrayLibrary.Array_AddUnique` (`self.LockOnTarget`) OtherActor))

(event `self.LockOnRadius.OnComponentEndOverlap`
  (params (OverlappedComponent :type "PrimitiveComponent Object Reference") (OtherActor :type "Actor Object Reference") (OtherComp :type "PrimitiveComponent Object Reference") (OtherBodyIndex :type Integer))
  (`KismetArrayLibrary.Array_RemoveItem` (`self.LockOnTarget`) OtherActor))

(fn `UserConstructionScript`)