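; BP_Triger is a win trigger volume that shows the WBP_WIn screen when its Box begins an overlap.
; The overlap switches input to UI-only and shows the cursor without checking which actor entered.
; It then casts the player character to BP_P1, adds the win widget to the viewport and hides the character's UiScreen through a 0.01-second timer event.
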(event `self.Box.OnComponentBeginOverlap`
  (params (OverlappedComponent :type "PrimitiveComponent Object Reference") (OtherActor :type "Actor Object Reference") (OtherComp :type "PrimitiveComponent Object Reference") (OtherBodyIndex :type Integer) (bFromSweep :type Boolean) (SweepResult :type "HitResult Structure (by ref)"))
  (`WidgetBlueprintLibrary.SetInputMode_UIOnlyEx` null null)
  (set `PlayerController.bShowMouseCursor` true (`GameplayStatics.GetPlayerController` 0))
  (bind _asbp_p1 (cast `/Game/KHJ/Blueprints/BP_P1` (`GameplayStatics.GetPlayerCharacter` 0)))
  (`KismetSystemLibrary.K2_SetTimerDelegate` (delegate `CustomEvent`) 0.01)
  (bind _returnvalue (`|GenericCreateObject` "/Game/KKW/UI/WBP_WIn.WBP_WIn_C"))
  (`UserWidget.AddToViewport` _returnvalue 0))

(event `CustomEvent`
  (`Widget.SetVisibility` (`/Game/KHJ/Blueprints/BP_P1.uiScreen` (stale `self.Box.OnComponentBeginOverlap` _asbp_p1)) "Hidden"))

(fn `UserConstructionScript`)