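; Test enemy AI that chases and attacks the player, built as an enum state machine run every Tick.
; Stay starts Chase when the player is near, and Chase uses SimpleMoveToLocation, selecting PowerAttack at close range.
; Attack, Skill and JumpSkill play timer-gated animations before returning to Chase; PowerAttack only bounces back, its animation unwired.
; Return, Die and Parry are empty stubs, and several branches are disconnected.
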(event `self.ReceiveBeginPlay`)

(event `Serching`
  ;[1 1 1] 초기 서칭
  (`/Engine/EditorBlueprintResources/StandardMacros.IsValid` (`GameplayStatics.GetPlayerCharacter` 0)
    (:`Is Valid`
      (set `self.State` "NewEnumerator3"))
    (:`Is Not Valid`
      (`KismetSystemLibrary.Delay` 0.1))))

(event `EventStay`
  (bind _returnvalue (`GameplayStatics.GetPlayerCharacter` 0))
  ;[1 1 1] 내 반경 20M안에 플레이어가 있다면 추적 상태로 전이하고싶다.
  (set `self.ChaseTarget` _returnvalue)
  (if (< (`KismetMathLibrary.Vector_Distance` (`self.K2_GetActorLocation` _returnvalue) (`self.K2_GetActorLocation`)) 2000.0)
    (set `self.State` "NewEnumerator0")))

(event `EventChase`
  (bind _returnvalue (`KismetMathLibrary.VSize` (- (`self.K2_GetActorLocation` (`GameplayStatics.GetPlayerCharacter` 0)) (`self.K2_GetActorLocation` self))))
  ;[1 1 1] 목적지를 향해 이동하고싶다.
  (`AIBlueprintHelperLibrary.SimpleMoveToLocation` (`self.GetController`) (`self.K2_GetActorLocation` (`self.ChaseTarget`)))
  (`|ExecutionSequence`
    (:`then_0`
      (if (> 500.0 (`KismetMathLibrary.VSize` (- (`self.K2_GetActorLocation` (`GameplayStatics.GetPlayerCharacter` 0)) (`self.K2_GetActorLocation` self))))
        (set `self.State` "NewEnumerator3")
        ;[1 1 1] 3중에 하나를 랜덤으로 공격하고 싶다.
        (switch `int` (`KismetMathLibrary.RandomIntegerInRange` 1 1)
          (:`1`
            (set `self.State` "NewEnumerator5")))))
    (:`then_1`
      (if (and (> 1000.0 _returnvalue) (> _returnvalue 500.0))
        (set `self.State` "NewEnumerator3")))))

(event `EventReturn`)

(event `EventAttack`
  ;[1 1 1] 가까이 왔을 때 일반 공격하고 싶다.
  (bind _output_get (set `self.CurrentTime1` (+ (`self.CurrentTime1`) (`GameplayStatics.GetWorldDeltaSeconds`))))
  (if (> _output_get (`self.MakeTime1`))
    (`SkeletalMeshComponent.PlayAnimation` (`self.Mesh`) "/Game/Asset/animation/Attack1_Jab.Attack1_Jab" false)
    (set `self.CurrentTime1` 0.0)
    (set `self.State` "NewEnumerator0")
    (else
      (set `self.State` "NewEnumerator0"))))

(event `Power Attack`
  ;[1 1 1] 가까이 왔을 때 쌔게 때리고 싶다
  (bind _output_get (set `self.CurrentTime2` (+ (`self.CurrentTime2`) (`GameplayStatics.GetWorldDeltaSeconds`))))
  (if (not (> _output_get (`self.MakeTime2`)))
    (set `self.State` "NewEnumerator0")))

(event `self.ReceiveTick`
  (params (DeltaSeconds :type "Float (single-precision)"))
  (switch `/Game/YWK/Blueprints/EEnemyState` (`self.State`)
    (:`NewEnumerator3`
      (`self.EventStay`))
    (:`NewEnumerator0`
      (`self.EventChase`))
    (:`NewEnumerator4`
      (`self.EventReturn`))
    (:`NewEnumerator1`
      (`self.EventAttack`))
    (:`NewEnumerator5`
      (`self.Power Attack`))
    (:`NewEnumerator6`
      (`self.Skill`))
    (:`NewEnumerator8`
      (`self.jump skill`))
    (:`NewEnumerator9`
      (`self.Serching`))
    (:`NewEnumerator10`
      (`self.Die`))))

(event `Skill`
  ;[1 1 1] 가까이 왔을 때 스킬을 쓰고 싶다.
  (bind _output_get (set `self.CurrentTime3` (+ (`self.CurrentTime3`) (`GameplayStatics.GetWorldDeltaSeconds`))))
  (if (> _output_get (`self.MakeTime3`))
    (`SkeletalMeshComponent.PlayAnimation` (`self.Mesh`) "/Game/Asset/animation/Attack3_Hook.Attack3_Hook" false)
    (set `self.CurrentTime3` 0.0)
    (set `self.State` "NewEnumerator0")
    (else
      (set `self.State` "NewEnumerator0"))))

(event `jump skill`
  ;[1 1 1] 스킬(점프해서 적을 찍는 모션-> 일정거리 떨어져 있을 때)
  (bind _output_get (set `self.CurrentTime4` (+ (`self.CurrentTime4`) (`GameplayStatics.GetWorldDeltaSeconds`))))
  (if (> _output_get (`self.makeTime4`))
    (`SkeletalMeshComponent.PlayAnimation` (`self.Mesh`) "/Game/Characters/Mannequins/Animations/Manny/MM_Jump.MM_Jump" false)
    (set `self.CurrentTime4` 0.0)
    (set `self.State` "NewEnumerator0")
    (else
      (set `self.State` "NewEnumerator0"))))

(event `Hit`
  ;[1 1 1] 맞을 때의 반응을 하고 싶다.
  (if (`self.HitbyPlayer`)
    (`SkeletalMeshComponent.SetAnimation` (`self.Mesh`) "/Game/YWK/makeAnimation/Down.Down")
    (set `self.State` "NewEnumerator0")
    (else
      (set `self.State` "NewEnumerator1"))))

(event `Die`)

(event `Parry`)

(fn `NewFunction`)

(fn `UserConstructionScript`)