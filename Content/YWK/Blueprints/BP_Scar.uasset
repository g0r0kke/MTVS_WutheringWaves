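; BP_Scar is a boss enemy with a Tick-driven state machine over Finding, Idle, Move and Attack.
; PawnSensing ends Finding, and distance checks drive Idle, chasing via AIMoveTo, and Attack.
; Attack runs only on the transition tick, since the steady-state check omits it, and just prints behind a cooldown.
; Random attack selection, heavy attack and skill logic are unconnected.
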(event `self.PawnSensing.OnSeePawn`
  (params (Pawn :type "Pawn Object Reference"))
  ;[1 1 1] Find
  (set `self.isSeeingPlayer` true))

(event `Following`
  (bind _returnvalue (`KismetMathLibrary.VSize` (- (`self.K2_GetActorLocation` (`GameplayStatics.GetPlayerCharacter` 0)) (`self.K2_GetActorLocation` self))))
  ;[1 1 1] Move
  (if (`self.isSeeingPlayer`)
    (`|AIMoveTo` self (0.0 0.0 0.0) (`GameplayStatics.GetPlayerCharacter` 0)
      (:`then`
        ;[1 1 1] 일정거리 지나면 멈추게
        (if (or (< _returnvalue 100.0) (> _returnvalue 400.0))
          (`NavMovementComponent.StopActiveMovement` (`self.CharacterMovement`))
          (set `self.NextState` "NewEnumerator0"))))))

(event `self.ReceiveTick`
  (params (DeltaSeconds :type "Float (single-precision)"))
  (bind _returnvalue (and (== (`KismetMathLibrary.Conv_ByteToInt` (`self.CurrentState`)) (`KismetMathLibrary.Conv_ByteToInt` (`self.NextState`))) (== (`KismetMathLibrary.Conv_ByteToInt` (`self.NextState`)) (`KismetMathLibrary.Conv_ByteToInt` (enumliteral `/Game/YWK/Blueprints/BP_Enum` "NewEnumerator0")))))
  (if (or (or (and (== (`KismetMathLibrary.Conv_ByteToInt` (`self.CurrentState`)) (`KismetMathLibrary.Conv_ByteToInt` (`self.NextState`))) (== (`KismetMathLibrary.Conv_ByteToInt` (`self.NextState`)) (`KismetMathLibrary.Conv_ByteToInt` (enumliteral `/Game/YWK/Blueprints/BP_Enum` "NewEnumerator1")))) _returnvalue) (or _returnvalue (and (== (`KismetMathLibrary.Conv_ByteToInt` (`self.CurrentState`)) (`KismetMathLibrary.Conv_ByteToInt` (`self.NextState`))) (== (`KismetMathLibrary.Conv_ByteToInt` (`self.NextState`)) (`KismetMathLibrary.Conv_ByteToInt` (enumliteral `/Game/YWK/Blueprints/BP_Enum` "NewEnumerator5"))))))
    (switch `/Game/YWK/Blueprints/BP_Enum` (`self.CurrentState`) :!label _label
      (:`NewEnumerator5`
        ;[1 1 1] Find
        (if (`self.isSeeingPlayer`)
          (set `self.NextState` "NewEnumerator0")
          ;[1 1 1] Move
          (set `self.CurrentState` "NewEnumerator0")))
      (:`NewEnumerator0`
        ;[1 1 1] Idle
        (if (not (> (`KismetMathLibrary.VSize` (- (`self.K2_GetActorLocation` (`GameplayStatics.GetPlayerCharacter` 0)) (`self.K2_GetActorLocation` self))) 300.0))
          (set `self.NextState` "NewEnumerator1")))
      (:`NewEnumerator1`
        (`self.Following`)
        ;[1 1 1] 공격 범위
        (if (<= (`KismetMathLibrary.VSize` (- (`self.K2_GetActorLocation` (`GameplayStatics.GetPlayerCharacter` 0)) (`self.K2_GetActorLocation` self))) 100.0)
          (set `self.NextState` "NewEnumerator2")))
      (:`NewEnumerator2`
        (`self.Attack`)))
    (elif (!= (`KismetMathLibrary.Conv_ByteToInt` (`self.CurrentState`)) (`KismetMathLibrary.Conv_ByteToInt` (`self.NextState`)))
      (set `self.CurrentState` (`self.NextState`))
      (goto _label))))

(event `self.ReceiveBeginPlay`
  ;[1 1 1] 보스 체력
  (set `self.CurrentState` "NewEnumerator5")
  (set `self.NextState` "NewEnumerator5")
  (set `self.HP` (`self.Max HP`)))

(event `Attack`
  ;[1 1 1] 일반 공격
  (`self.normal CoolTime` (`self.CurrentTime`) (`GameplayStatics.GetWorldDeltaSeconds`) (`self.MakeTime(nor)`))
  (if (<= (`self.CurrentTime`) 0.0)
    (`KismetSystemLibrary.PrintString` "Attack!")
    (set `self.CurrentTime` (`self.MakeTime(skill)`))
    (if (>= (`KismetMathLibrary.VSize` (- (`self.K2_GetActorLocation` (`GameplayStatics.GetPlayerCharacter` 0)) (`self.K2_GetActorLocation` self))) 100.0)
      _)))

(fn `Hard CoolTime`
  (params (CurrentTime2 :type "Float (double-precision)") (DeltaTime :type "Float (double-precision)") (`MakeTime(hard)` :type "Float (double-precision)"))
  (if (< 0.0 `MakeTime(hard)`)
    (set `self.CurrentTime2` (- CurrentTime2 DeltaTime))))

(fn `normal CoolTime`
  (params (CurrentTime :type "Float (double-precision)") (DeltaTime :type "Float (double-precision)") (MakeTime :type "Float (double-precision)"))
  (set `self.CurrentTime` (- CurrentTime DeltaTime)))

(fn `Skill CoolTime`
  (params (CurrentTime3 :type "Float (double-precision)") (DeltaTime :type "Float (double-precision)") (`MakeTime(skill)` :type "Float (double-precision)"))
  (if (< 0.0 `MakeTime(skill)`)
    (set `self.CurrentTime3` (- CurrentTime3 DeltaTime))))

(fn `UserConstructionScript`)