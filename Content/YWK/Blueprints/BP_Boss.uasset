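; Boss character with montage-driven melee attacks, a jump skill, HP and a stun-then-destroy death.
; Attack, damage and parry-window events relay through dispatchers, while helper functions expose patrol route and walk speed.
; Damage arrives by binding to the player weapon's OnP1Attack shortly after BeginPlay.
; A hit during an attack flagged IsParrying triggers a reaction montage, then a random hand, kick or jump-kick attack after a delay.
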(event `self.ReceiveBeginPlay`
  ;[1 1 1] 보스 첫 상태
  (`|ExecutionSequence`
    (:`then_0`
      (`self.AttackFoot`))
    (:`then_1`
      (set `self.HP` (`self.MaxHP`)))
    (:`then_2`
      (`KismetSystemLibrary.Delay` 0.2)
      (`self.DamageProcess`))))

(event `AttackHand`
  ;[1 1 1] 일반공격
  (set `self.IsParrying` true)
  (`|PlayMontage` (`self.Mesh`) "/Game/YWK/Rig/Standing_Melee_Attack_Horizontal_Montage.Standing_Melee_Attack_Horizontal_Montage"
    (:`OnCompleted`
      (set `self.Attackbyplayer` false)
      (set `self.IsParrying` false))))

(event `JumpKick`
  ;[1 1 1] 일반공격
  (set `self.IsParrying` true)
  (`|PlayMontage` (`self.Mesh`) "/Game/YWK/Rig/Flying_Kick_Montage.Flying_Kick_Montage" 0.7
    (:`OnCompleted`
      (set `self.Attackbyplayer` false)
      (set `self.IsParrying` false))))

(event `AttackKick`
  ;[1 1 1] 일반공격
  (set `self.IsParrying` true)
  (`|PlayMontage` (`self.Mesh`) "/Game/YWK/Rig/Kick1_Montage.Kick1_Montage" 1.3
    (:`OnCompleted`
      (set `self.Attackbyplayer` false)
      (set `self.IsParrying` false))))

(event `Deal1`
  ;[1 1 1] 일반공격
  (`self.OnAttackEnd` 10))

(event `AttackFoot`
  ;[1 1 1] 일반공격
  (set `self.IsAttackFoot` true))

(event `Skill1`
  ;[1 1 1] 스킬공격
  (`|PlayMontage` (`self.Mesh`) "/Game/YWK/makeAnimation/jumpskill.jumpskill" 1.2))

(event `Attack Start`
  ;[1 1 1] 스킬공격
  (`self.OnAttackStart`))

(event `DamageProcess`
  ;[1 1 1] 피격 로직
  (bind _returnvalue (`GameplayStatics.GetActorOfClass` "/Game/KHJ/Blueprints/BP_Player1Weapon.BP_Player1Weapon_C"))
  (add `/Game/KHJ/Blueprints/BP_Player1Weapon.OnP1Attack` _returnvalue (delegate `DamagedByPlayer`)))

(event `Parry Timing Start`
  ;[1 1 1] 패링
  (`self.OnParryAttackStart`))

(event `Parry Timing End`
  ;[1 1 1] 패링
  (`self.OnParryAttackEnd` 0))

(event `DamagedByPlayer`
  (params (Damage :type Integer))
  ;[1 1 1] 피격 로직
  ;;[1 1 1] 체력 깎임
  (set `self.HP` (- (`self.HP`) Damage))
  (if (<= (`self.HP`) 0.0)
    (`/Engine/EditorBlueprintResources/StandardMacros.DoOnce` false
      (:`Completed`
        (`self.Death`)))
    (else
      (set `self.Attackbyplayer` true)
      (if (`self.IsParrying`)
        (`self.Parry`)))))

(event `self.ReceiveTick`
  (params (DeltaSeconds :type "Float (single-precision)")))

(event `Parry`
  ;[1 1 1] 피격 로직
  ;[1 1 1] 패링
  (`|PlayMontage` (`self.Mesh`) "/Game/YWK/animation/Backflip/NewRig/Attack_by_player.Attack_by_player"
    (:`OnCompleted`
      (set `self.Attackbyplayer` false)
      (`KismetSystemLibrary.Delay` 2.0)
      (switch `int` (`KismetMathLibrary.RandomIntegerInRange` 0 2)
        (:`0`
          (`self.AttackHand`))
        (:`1`
          (`self.AttackKick`))
        (:`2`
          (`self.JumpKick`))))))

(event `Death`
  ;[1 1 1] 죽음
  (bind _returnvalue (`self.PlayAnimMontage` "/Game/YWK/makeAnimation/Stunned_Montage.Stunned_Montage"))
  (`KismetSystemLibrary.Delay` (- _returnvalue 0.6))
  (`ActorComponent.SetComponentTickEnabled` (`self.Mesh`) false)
  (`self.K2_DestroyActor`))

(fn `Get Mesh`
  (returns (NewParam :type "SkeletalMeshComponent Object Reference"))
  (return (`self.Mesh`)))

(fn `GetPatrolRute`
  (returns (PatrolRute :type "/Game/YWK/Blueprints/AI/BP_PatrolRute Object Reference"))
  (return (`self.PatrolRute`)))

(fn `LoseHealth`
  (set `self.HP` (- (`self.HP`) 1.0)))

(fn `SetMovementSpeed`
  (params (Speed :type "/Game/YWK/Blueprints/AI/Decorators/E_MovementSpeed Enum" :default "NewEnumerator0"))
  (returns (SpeedValue :type "Float (double-precision)"))
  (bind _output_get (set `CharacterMovementComponent.MaxWalkSpeed` (select `/Game/YWK/Blueprints/AI/Decorators/E_MovementSpeed` Speed :`NewEnumerator1` 100.0 :`NewEnumerator2` 300.0 :`NewEnumerator3` 500.0 :!type "Float (single-precision)") (`self.CharacterMovement`)))
  (return _output_get))

(fn `UserConstructionScript`)