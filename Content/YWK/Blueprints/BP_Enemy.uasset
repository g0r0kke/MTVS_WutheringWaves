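; BP_Enemy is a melee enemy that chases and attacks the player.
; When PawnSensing sees a BP_CPlayer1, it moves to it via AIMoveTo and plays a horizontal melee montage, limited by a DoOnce that resets after a delay.
; A separate Damage_Player event, not called in this graph, applies damage to the player character if the BPMonsterCard child actor is a BP_MonsterCard, without checking range or hit.
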(event `self.PawnSensing.OnSeePawn`
  (params (Pawn :type "Pawn Object Reference"))
  (bind _asbp_cplayer_1 (cast `/Game/KHJ/Blueprints/BP_CPlayer1` Pawn))
  (`|AIMoveTo` self (0.0 0.0 0.0) _asbp_cplayer_1 100.0
    (:`OnSuccess`
      (`/Engine/EditorBlueprintResources/StandardMacros.DoOnce` false :!label _label
        (:`Completed`
          (`self.PlayAnimMontage` "/Game/YWK/makeAnimation/Standing_Melee_Attack_Horizontal_Montage.Standing_Melee_Attack_Horizontal_Montage")
          (`KismetSystemLibrary.Delay` 5.0)
          (goto _label :!via `Reset`))))))

(event `Damage_Player`
  ;[1 1 1] 무기로 데미지 주기
  (cast `/Game/YWK/Blueprints/BP_MonsterCard` (`ChildActorComponent.ChildActor` (`self.BP_MonsterCard`)))
  (bind _asbp_cplayer_1 (cast `/Game/KHJ/Blueprints/BP_CPlayer1` (`GameplayStatics.GetPlayerCharacter` 0)))
  (`GameplayStatics.ApplyDamage` _asbp_cplayer_1 0.0 null self))

(fn `UserConstructionScript`)