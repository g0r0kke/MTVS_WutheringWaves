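; BP_JumpBack is an anim notify state that moves BP_Boss during an animation, named as a backward jump.
; Each tick casts the mesh owner to BP_Boss and lerps its location toward Endlocation plus the constant world backward vector, using frame delta as alpha and no sweep.
; Endlocation is never set here, and NotifyBegin and NewFunction are empty apart from disconnected leftover nodes.
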(fn `NewFunction`)

(fn `Received_NotifyBegin`
  (params (MeshComp :type "SkeletalMeshComponent Object Reference") (Animation :type "AnimSequenceBase Object Reference") (TotalDuration :type "Float (single-precision)") (EventReference :type "AnimNotifyEventReference Structure (by ref)"))
  (returns (ReturnValue :type Boolean)))

(fn `Received_NotifyTick`
  (params (MeshComp :type "SkeletalMeshComponent Object Reference") (Animation :type "AnimSequenceBase Object Reference") (FrameDeltaTime :type "Float (single-precision)") (EventReference :type "AnimNotifyEventReference Structure (by ref)"))
  (returns (ReturnValue :type Boolean))
  (bind _asbp_boss (cast `/Game/YWK/Blueprints/BP_Boss` (`ActorComponent.GetOwner` MeshComp)))
  (`Actor.K2_SetActorLocation` _asbp_boss (`KismetMathLibrary.VLerp` (`Actor.K2_GetActorLocation` (`CharacterMovementComponent.GetCharacterOwner` (`Character.CharacterMovement` _asbp_boss))) (+ (`KismetMathLibrary.Vector_Backward`) (`self.Endlocation`)) FrameDeltaTime) false false)
  (return false))