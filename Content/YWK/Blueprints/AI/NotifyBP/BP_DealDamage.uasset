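; BP_DealDamage is an animation notify state that triggers the boss's attack during an animation.
; On begin, it casts the mesh owner to BP_Boss and calls Attack when the Right_FootSocket is within a fixed distance of the world origin.
; The distance check uses a zero vector, with no reference to a target actor.
; The end event only performs the boss cast and has no further effect.
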(fn `Received_NotifyBegin`
  (params (MeshComp :type "SkeletalMeshComponent Object Reference") (Animation :type "AnimSequenceBase Object Reference") (TotalDuration :type "Float (single-precision)") (EventReference :type "AnimNotifyEventReference Structure (by ref)"))
  (returns (ReturnValue :type Boolean))
  (bind _asbp_boss (cast `/Game/YWK/Blueprints/BP_Boss` (`ActorComponent.GetOwner` MeshComp)))
  (if (>= 100.0 (`KismetMathLibrary.Vector_Distance` (`SceneComponent.GetSocketLocation` MeshComp "Right_FootSocket")))
    (`/Game/YWK/Blueprints/BP_Boss.Attack` _asbp_boss)
    (return false)))

(fn `Received_NotifyEnd`
  (params (MeshComp :type "SkeletalMeshComponent Object Reference") (Animation :type "AnimSequenceBase Object Reference") (EventReference :type "AnimNotifyEventReference Structure (by ref)"))
  (returns (ReturnValue :type Boolean))
  (cast `/Game/YWK/Blueprints/BP_Boss` (`ActorComponent.GetOwner` MeshComp))
  (return false))