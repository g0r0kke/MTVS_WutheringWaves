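; AIC_Enemy_Base is a base AI controller for enemies that runs the BT_Enemy_Base behavior tree when it possesses a pawn.
; Helper functions drive the tree through the blackboard by writing a Boss_State enum to the state key.
; SetStateOfAttacking also stores the attack target object.
; Both the passive and attacking setters currently write the same enum entry, so the state value does not distinguish them.
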(event `self.ReceivePossess`
  (params (PossessedPawn :type "Pawn Object Reference"))
  (`self.RunBehaviorTree` "/Game/YWK/Blueprints/AI/BT_Enemy_Base.BT_Enemy_Base"))

(fn `SetStateOfAttacking`
  (params (AttackTarget :type "Actor Object Reference"))
  (`BlackboardComponent.SetValueAsObject` (`self.Blackboard`) (`self.AttackTarget Key Name`) AttackTarget)
  (`BlackboardComponent.SetValueAsEnum` (`self.Blackboard`) (`self.State Key Name`) (enumliteral `/Game/YWK/Blueprints/AI/Decorators/Boss_State` "NewEnumerator4")))

(fn `SetStateOfPassive`
  (`BlackboardComponent.SetValueAsEnum` (`self.Blackboard`) (`self.State Key Name`) (enumliteral `/Game/YWK/Blueprints/AI/Decorators/Boss_State` "NewEnumerator4")))

(fn `UserConstructionScript`)