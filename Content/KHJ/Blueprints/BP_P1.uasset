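; Player character Blueprint for a melee boss fight, handling attack, dash, roll and just-avoid actions, plus HP display and defeat screen.
; Actions play montages, usually lock input on a timer and often shake the camera.
; Tick rebinds boss and weapon events every frame, driving hit reactions and spawned damage indicators.
; Boss attack windows enable slow-motion dodges; attacking as a parry attack ends counts as a parry.
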(event `self.ReceiveBeginPlay`
  ;[1 1 1] 체력, 죽음
  (bind _returnvalue (`|CreateWidget` "/Game/KHJ/UI/WB_PlayerHP.WB_PlayerHP_C"))
  (set `self.uiScreen` _returnvalue)
  (`UserWidget.AddToViewport` (`self.uiScreen`) 0)
  (`KismetSystemLibrary.Delay` 0.05)
  (`self.UIctrlHP`))

(event `self.DashStart`
  ;[1 1 1] 이동
  (`self.PlayAnimMontage` "/Game/KHJ/Animations/Rover/AM_RUN_Montage.AM_RUN_Montage" 0.8)
  (`GameplayStatics.PlayWorldCameraShake` "/Game/KHJ/Blueprints/CS_FOVO2.CS_FOVO2_C" (`self.K2_GetActorLocation`) 0.0 500.0)
  (`self.DisableInput` null)
  (`KismetSystemLibrary.K2_SetTimer` null "EnablePlayerInput" 0.2))

(event `self.P1Death`
  (bind _returnvalue (`GameplayStatics.GetPlayerController` 0))
  ;[1 1 1] 체력, 죽음
  (`self.PlayAnimMontage` "/Game/KHJ/Animations/Rover/AM_two_handed_sword_death.AM_two_handed_sword_death" 0.8)
  (`self.DisableInput` null)
  (`KismetSystemLibrary.K2_SetTimer` null "EnablePlayerInput" 2.0)
  (`KismetSystemLibrary.PrintString` "플레이어 사망")
  (`KismetSystemLibrary.Delay` 2.0)
  (`WidgetBlueprintLibrary.SetInputMode_UIOnlyEx` _returnvalue null)
  (set `PlayerController.bShowMouseCursor` true _returnvalue)
  (bind _returnvalue_2 (`|GenericCreateObject` "/Game/KKW/UI/WBP_Defeat.WBP_Defeat_C"))
  (`UserWidget.AddToViewport` _returnvalue_2 0))

(event `self.Roll1Start`
  ;[1 1 1] 이동
  (`self.PlayAnimMontage` "/Game/KHJ/Animations/Rover/AM_Frontflip.AM_Frontflip" 1.5)
  (`self.DisableInput` null)
  (`KismetSystemLibrary.K2_SetTimer` null "EnablePlayerInput" 0.5))

(event `self.Roll2Start`
  ;[1 1 1] 이동
  (`self.PlayAnimMontage` "/Game/KHJ/Animations/Rover/AM_Backflip.AM_Backflip" 1.5)
  (`self.DisableInput` null)
  (`KismetSystemLibrary.K2_SetTimer` null "EnablePlayerInput" 0.5))

(event `self.JustAvoidStart`
  ;[1 1 1] 저스트 회피
  (if (`self.IsBossAttack`)
    (set `self.IsAvoid` true)
    (`GameplayStatics.SetGlobalTimeDilation` 0.5)
    (`self.PlayAnimMontage` "/Game/KHJ/Animations/Rover/AM_Backflip.AM_Backflip" 1.3)
    (`GameplayStatics.PlayWorldCameraShake` "/Game/KHJ/Blueprints/CS_FOVO2.CS_FOVO2_C" (`self.K2_GetActorLocation`) 0.0 500.0)
    (`self.DisableInput` null)
    (`KismetSystemLibrary.Delay` 0.4)
    (`GameplayStatics.SetGlobalTimeDilation` 1.2)
    (`KismetSystemLibrary.K2_SetTimer` null "EnablePlayerInput" 0.5)
    (`KismetSystemLibrary.Delay` 0.5)
    (`GameplayStatics.SetGlobalTimeDilation` 1.0)
    (`KismetSystemLibrary.Delay` 2.1)
    (set `self.IsAvoid` false)
    (`KismetSystemLibrary.PrintString` "끝")
    (else
      (`self.PlayAnimMontage` "/Game/KHJ/Animations/Rover/AM_BackRun_Montage.AM_BackRun_Montage" 0.8)
      (`self.DisableInput` null)
      (`KismetSystemLibrary.K2_SetTimer` null "EnablePlayerInput" 0.2))))

(event `self.Attack1Start`
  ;[1 1 1] 공격
  (set `self.bIsAttack` true)
  (`self.PlayAnimMontage` "/Game/KHJ/Animations/Rover/AM_attack1.AM_attack1" 1.5)
  (`self.DisableInput` null)
  (`KismetSystemLibrary.K2_SetTimer` null "EnablePlayerInput" 0.4)
  (`GameplayStatics.PlayWorldCameraShake` "/Game/KHJ/Blueprints/CS_FOVO1.CS_FOVO1_C" (`self.K2_GetActorLocation`) 0.0 500.0)
  (`KismetSystemLibrary.Delay` 0.4)
  (set `self.bIsAttack` false))

(event `self.Attack2Start`
  ;[1 1 1] 공격
  (set `self.bIsAttack` true)
  (`self.PlayAnimMontage` "/Game/KHJ/Animations/Rover/AM_attack2.AM_attack2" 1.5)
  (`self.DisableInput` null)
  (`KismetSystemLibrary.K2_SetTimer` null "EnablePlayerInput" 0.4)
  (`GameplayStatics.PlayWorldCameraShake` "/Game/KHJ/Blueprints/CS_FOVO2.CS_FOVO2_C" (`self.K2_GetActorLocation`) 0.0 500.0)
  (`KismetSystemLibrary.Delay` 0.4)
  (set `self.bIsAttack` false))

(event `self.ReceiveTick`
  (params (DeltaSeconds :type "Float (single-precision)"))
  (`|ExecutionSequence`
    (:`then_0`
      (bind _returnvalue (`GameplayStatics.GetActorOfClass` "/Game/YWK/Blueprints/BP_Boss.BP_Boss_C"))
      (`/Engine/EditorBlueprintResources/StandardMacros.IsValid` _returnvalue
        (:`Is Valid`
          (bind _returnvalue_2 (`GameplayStatics.GetActorOfClass` "/Game/YWK/Blueprints/BP_Boss.BP_Boss_C"))
          (`|ExecutionSequence`
            (:`then_0`
              ;[1 1 1] 일반 공격
              (add `/Game/YWK/Blueprints/BP_Boss.OnAttackStart` _returnvalue_2 (delegate `BossAttack`)))
            (:`then_1`
              (add `/Game/YWK/Blueprints/BP_Boss.OnAttackEnd` _returnvalue_2 (delegate `BossAttackEnd`)))
            (:`then_2`
              ;[1 1 1] 패링 공격
              (add `/Game/YWK/Blueprints/BP_Boss.OnParryAttackStart` _returnvalue_2 (delegate `ParryAttack`)))
            (:`then_3`
              (add `/Game/YWK/Blueprints/BP_Boss.OnParryAttackEnd` _returnvalue_2 (delegate `ParryAttackEnd`)))))))
    (:`then_1`
      ;[1 1 1] Damage UI
      (bind _returnvalue_3 (`GameplayStatics.GetActorOfClass` "/Game/KHJ/Blueprints/BP_Player1Weapon.BP_Player1Weapon_C"))
      (add `/Game/KHJ/Blueprints/BP_Player1Weapon.OnP1Attack` _returnvalue_3 (delegate `CustomEvent`)))))

(event `BossAttack`
  ;[1 1 1] 일반 공격
  (set `self.IsBossAttack` true))

(event `BossAttackEnd`
  (params (Damage :type Integer))
  ;[1 1 1] 일반 공격
  (if (`self.IsAvoid`)
    (`KismetSystemLibrary.PrintString` "회피 성공!")
    (else
      (`self.PlayAnimMontage` "/Game/KHJ/Animations/Rover/AM_Hurt.AM_Hurt")
      (`self.OnHitEvent` Damage)
      (`self.UIctrlHP`)
      (set `self.IsBossAttack` false)
      (`self.HideWeapon`)
      (`self.DisableInput` null)
      (`KismetSystemLibrary.K2_SetTimer` null "EnablePlayerInput" 1.5))))

(event `self.Attack3Start`
  (bind _returnvalue (`self.K2_GetActorLocation`))
  ;[1 1 1] 공격
  (set `self.bIsAttack` true)
  (`self.PlayAnimMontage` "/Game/KHJ/Animations/Rover/AM_attack3.AM_attack3" 1.5)
  (`self.DisableInput` null)
  (`KismetSystemLibrary.K2_SetTimer` null "EnablePlayerInput" 0.4)
  (`GameplayStatics.PlayWorldCameraShake` "/Game/KHJ/Blueprints/CS_FOVO1.CS_FOVO1_C" _returnvalue 0.0 500.0)
  (`GameplayStatics.PlayWorldCameraShake` "/Game/KHJ/Blueprints/CS_FOVO2.CS_FOVO2_C" _returnvalue 0.0 500.0)
  (`KismetSystemLibrary.Delay` 0.4)
  (set `self.bIsAttack` false))

(event `ParryAttack`
  ;[1 1 1] 패링 공격
  (set `self.IsBossAttack` true))

(event `self.Attack4Start`
  ;[1 1 1] 공격
  (set `self.bIsAttack` true)
  (`self.PlayAnimMontage` "/Game/KHJ/Animations/Rover/AM_attack4.AM_attack4" 1.5)
  (`self.DisableInput` null)
  (`KismetSystemLibrary.K2_SetTimer` null "EnablePlayerInput" 0.4)
  (`GameplayStatics.PlayWorldCameraShake` "/Game/KHJ/Blueprints/CS_FOVO4.CS_FOVO4_C" (`self.K2_GetActorLocation`) 0.0 500.0)
  (`KismetSystemLibrary.Delay` 0.4)
  (set `self.bIsAttack` false))

(event `ParryAttackEnd`
  (params (Damage :type Integer))
  ;[1 1 1] 패링 공격
  (if (`KismetMathLibrary.BooleanNOR` (`self.IsAvoid`) (`self.bIsAttack`))
    (`self.PlayAnimMontage` "/Game/KHJ/Animations/Rover/AM_Falling_Down.AM_Falling_Down")
    (`self.OnHitEvent` Damage)
    (`self.UIctrlHP`)
    (set `self.IsBossAttack` false)
    (`self.DisableInput` null)
    (`KismetSystemLibrary.K2_SetTimer` null "EnablePlayerInput" 1.5)
    (elif (`self.IsAvoid`)
      (`KismetSystemLibrary.PrintString` "회피 성공!")
      (elif (`self.bIsAttack`)
        (`KismetSystemLibrary.PrintString` "패링 성공!")
        (`GameplayStatics.SetGlobalTimeDilation` 0.5)
        (`KismetSystemLibrary.Delay` 0.5)
        (`GameplayStatics.SetGlobalTimeDilation` 1.0)
        (set `self.bIsAttack` false)))))

(event `self.StrongAttackStart`
  ;[1 1 1] 공격
  (set `self.bIsAttack` true)
  (`self.PlayAnimMontage` "/Game/KHJ/Animations/Rover/AM_strongattack.AM_strongattack" 1.2)
  (`self.DisableInput` null)
  (`KismetSystemLibrary.K2_SetTimer` null "EnablePlayerInput" 0.2)
  (`GameplayStatics.PlayWorldCameraShake` "/Game/KHJ/Blueprints/CS_FOVO4.CS_FOVO4_C" (`self.K2_GetActorLocation`) 0.0 500.0)
  (`KismetSystemLibrary.Delay` 0.4)
  (set `self.bIsAttack` false))

(event `CustomEvent`
  (params (Damage :type Integer))
  ;[1 1 1] Damage UI
  (bind (_up_vector _right_vector) (message `/Game/KHJ/Blueprints/BPI_Player.IF_GetVectors` (`GameplayStatics.GetPlayerCharacter` 0)))
  (`|SpawnActorFromClass` "/Game/KHJ/Blueprints/BP_DamageInd.BP_DamageInd_C" (`KismetMathLibrary.MakeTransform` (+ (* _up_vector 50.0) (* _right_vector 50.0) (`SceneComponent.GetSocketLocation` (`self.Mesh`) "NeckSocket"))) "Undefined" "MultiplyWithRoot" null (`KismetMathLibrary.Conv_IntToDouble` Damage) null))

(event `self.SkillStart`
  ;[1 1 1] 공격
  (set `self.bIsAttack` true)
  (`self.PlayAnimMontage` "/Game/KHJ/Animations/Rover/AM_attack3.AM_attack3" 1.5)
  (`self.DisableInput` null)
  (`KismetSystemLibrary.K2_SetTimer` null "EnablePlayerInput" 0.4)
  (`GameplayStatics.PlayWorldCameraShake` "/Game/KHJ/Blueprints/CS_FOVO1.CS_FOVO1_C" (`self.K2_GetActorLocation`) 0.0 500.0)
  (`KismetSystemLibrary.Delay` 0.4)
  (set `self.bIsAttack` false))

(event `self.AerialAttackStart`
  ;[1 1 1] 공격
  (set `self.bIsAttack` true)
  (`self.PlayAnimMontage` "/Game/KHJ/Animations/Rover/AM_JumpAttack.AM_JumpAttack" 1.5)
  (`self.DisableInput` null)
  (`KismetSystemLibrary.K2_SetTimer` null "EnablePlayerInput" 0.4)
  (`GameplayStatics.PlayWorldCameraShake` "/Game/KHJ/Blueprints/BP_CamShakeRot.BP_CamShakeRot_C" (`self.K2_GetActorLocation`) 0.0 1000.0)
  (`KismetSystemLibrary.Delay` 0.4)
  (set `self.bIsAttack` false))

(fn `EnablePlayerInput`
  (`self.EnableInput` null))

(fn `IF_GetVectors`
  (returns (`Up Vector` :type "Vector Structure") (`Right Vector` :type "Vector Structure"))
  (bind _returnvalue (`self.K2_GetActorRotation`))
  (return (`KismetMathLibrary.GetUpVector` _returnvalue) (`KismetMathLibrary.GetRightVector` _returnvalue)))

(fn `UIctrlHP`
  (bind _uiscreen (`self.uiScreen`))
  (set `/Game/KHJ/UI/WB_PlayerHP.hpRatio` (/ (`KismetMathLibrary.Conv_IntToDouble` (`self.HP`)) (`KismetMathLibrary.Conv_IntToDouble` (`self.InitialHP`))) _uiscreen)
  (set `/Game/KHJ/UI/WB_PlayerHP.hpString` (`KismetStringLibrary.Concat_StrStr` (`KismetStringLibrary.Conv_IntToString` (`self.HP`)) "/" (`KismetStringLibrary.Conv_IntToString` (`self.InitialHP`))) _uiscreen))

(fn `UserConstructionScript`)