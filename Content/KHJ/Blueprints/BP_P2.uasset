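; BP_P2 is a player character Blueprint with a gunplay montage attack and an enemy target lock.
; The lock input sphere-traces for Pawns along a direction derived from the camera's world location, not its rotation, and stores the hit actor.
; Tick turns the control rotation toward that actor with a downward pitch offset.
; No path releases the lock, and the looping timer set on a hit has no event bound.
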(event `self.Attack1Start`
  (`self.PlayAnimMontage` "/Game/KHJ/Animations/Gunplay_Montage.Gunplay_Montage" 1.5))

(event `TargetLock`
  (bind _returnvalue (`self.K2_GetActorLocation`))
  (if (`self.IsTargetLock`)
    (set `self.IsTargetLock` true)
    (else
      (set `self.IsTargetLock` true)
      (bind (_outhit _returnvalue_2) (`KismetSystemLibrary.SphereTraceSingleForObjects` :`Start` _returnvalue :`End` (+ (* (`KismetMathLibrary.GetForwardVector` (`KismetMathLibrary.Conv_VectorToRotator` (`SceneComponent.K2_GetComponentLocation` (`self.FollowCamera`)))) 600.0) _returnvalue) :`Radius` 200.0 :`ObjectTypes` (`|MakeArray` "ObjectTypeQuery3" :!type "EObjectTypeQuery Enum") :`DrawDebugType` "ForDuration"))
      (if _returnvalue_2
        (set `self.HItActor` (`.HitActor` (`GameplayStatics.BreakHitResult` _outhit)))
        (`KismetSystemLibrary.K2_SetTimerDelegate` :`Time` (`GameplayStatics.GetWorldDeltaSeconds`) :`bLooping` true)))))

(event `EnhancedInput|/Game/KKW/Input/IA_TargetLock`
  (params (ActionValue :type Boolean) (ElapsedSeconds :type "Float (double-precision)") (TriggeredSeconds :type "Float (double-precision)") (InputAction :type "InputAction Object Reference" :default "/Game/KKW/Input/IA_TargetLock.IA_TargetLock"))
  (:`Started`
    (`self.TargetLock`)))

(event `self.ReceiveTick`
  (params (DeltaSeconds :type "Float (single-precision)"))
  (bind (_returnvalue_roll _returnvalue_pitch _returnvalue_yaw) (`KismetMathLibrary.BreakRotator` (`KismetMathLibrary.FindLookAtRotation` (`self.K2_GetActorLocation`) (`self.K2_GetActorLocation` (`self.HItActor`)))))
  (`self.HItActor`
    (:`then`
      (`Controller.SetControlRotation` (`self.GetController`) (`KismetMathLibrary.MakeRotator` _returnvalue_roll (- _returnvalue_pitch 25.0) _returnvalue_yaw)))
    (:`else`)))

(event `lockenemy`)

(fn `UserConstructionScript`)