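; Player character Blueprint that handles third-person movement, camera look, jump, dash and avoid through Enhanced Input.
; BeginPlay adds the IMC_ThirdPerson mapping context; move follows control rotation and look supports per-axis inversion.
; Dash launches the character along its scaled horizontal velocity, gated by a timed flag.
; Avoid works only when stationary, instantly shifting the actor forward without sweep, with a DoOnce and Delay cooldown.
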(event `EnhancedInput|/Game/KHJ/EnhancedInput/INP_Avoid`
  (params (ActionValue :type Boolean) (ElapsedSeconds :type "Float (double-precision)") (TriggeredSeconds :type "Float (double-precision)") (InputAction :type "InputAction Object Reference" :default "/Game/KHJ/EnhancedInput/INP_Avoid.INP_Avoid"))
  (:`Triggered`
    ;[1 1 1] Avoid
    (if (== (`self.GetVelocity`) (0.0 0.0 0.0))
      (`/Engine/EditorBlueprintResources/StandardMacros.DoOnce` false :!label _label
        (:`Completed`
          (`self.K2_SetActorLocation` (+ (`self.K2_GetActorLocation`) (* (`self.GetActorForwardVector`) (`self.Speed`))))
          (`KismetSystemLibrary.Delay` 0.5)
          (goto _label :!via `Reset`))))))

(event `self.ReceiveBeginPlay`
  (bind _returnvalue (pcsubsystem `EnhancedInputLocalPlayerSubsystem` (`GameplayStatics.GetPlayerController` 0)))
  (`/Engine/EditorBlueprintResources/StandardMacros.IsValid` _returnvalue
    (:`Is Valid`
      (`EnhancedInputSubsystemInterface.AddMappingContext` _returnvalue "/Game/KHJ/EnhancedInput/IMC_ThirdPerson.IMC_ThirdPerson" 0 (struct)))))

(event `EnhancedInput|/Game/KHJ/EnhancedInput/INP_Dash`
  (params (ActionValue :type Boolean) (ElapsedSeconds :type "Float (double-precision)") (TriggeredSeconds :type "Float (double-precision)") (InputAction :type "InputAction Object Reference" :default "/Game/KHJ/EnhancedInput/INP_Dash.INP_Dash"))
  (bind (_returnvalue_x _returnvalue_y) (`KismetMathLibrary.BreakVector` (* (`self.GetVelocity`) 4.0)))
  ;[1 1 1] Dash
  (:`Triggered`
    (if (not (`self.IsDashing`))
      (set `self.IsDashing` true)
      (`self.LaunchCharacter` (`KismetMathLibrary.MakeVector` _returnvalue_x _returnvalue_y))
      (`KismetSystemLibrary.Delay` 0.5)
      (set `self.IsDashing` false))))

(event `EnhancedInput|/Game/KHJ/EnhancedInput/INP_Jump`
  (params (ActionValue :type Boolean) (ElapsedSeconds :type "Float (double-precision)") (TriggeredSeconds :type "Float (double-precision)") (InputAction :type "InputAction Object Reference" :default "/Game/KHJ/EnhancedInput/INP_Jump.INP_Jump"))
  (:`Started`
    (`self.Jump`))
  (:`Completed`
    (`self.StopJumping`)))

(event `EnhancedInput|/Game/KHJ/EnhancedInput/INP_Move`
  (params (ActionValue :type "Vector2D Structure") (ElapsedSeconds :type "Float (double-precision)") (TriggeredSeconds :type "Float (double-precision)") (InputAction :type "InputAction Object Reference" :default "/Game/KHJ/EnhancedInput/INP_Move.INP_Move"))
  (bind (_returnvalue_roll _returnvalue_pitch _returnvalue_yaw) (`KismetMathLibrary.BreakRotator` (`self.GetControlRotation`)))
  (:`Triggered`
    (`self.AddMovementInput` (`KismetMathLibrary.GetRightVector` (`self.GetControlRotation`)) ActionValue_X)
    (`self.AddMovementInput` (`KismetMathLibrary.GetForwardVector` (`KismetMathLibrary.MakeRotator` _returnvalue_roll 0.0 _returnvalue_yaw)) ActionValue_Y)))

(event `EnhancedInput|/Game/KHJ/EnhancedInput/INP_Look`
  (params (ActionValue :type "Vector2D Structure") (ElapsedSeconds :type "Float (double-precision)") (TriggeredSeconds :type "Float (double-precision)") (InputAction :type "InputAction Object Reference" :default "/Game/KHJ/EnhancedInput/INP_Look.INP_Look"))
  (:`Triggered`
    (`self.AddControllerYawInput` (* ActionValue_X (`KismetMathLibrary.SelectFloat` -1.0 1.0 (`self.InvertCameraX`))))
    (`self.AddControllerPitchInput` (* ActionValue_Y (`KismetMathLibrary.SelectFloat` -1.0 1.0 (`self.InvertCameraY`))))))

(fn `UserConstructionScript`)